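; BP_Skill_Warp is a warp skill Blueprint that shows a ground-targeting decal under the mouse cursor; the file itself contains no teleport logic.
; Each tick, GetCursorLocation traces WorldStatic objects under the cursor, placing the decal at the hit and aligning it to the surface normal, or hiding it on a miss.
; Spell calls the parent, locks the owner's movement and plays a buff montage, and EndSpell restores movement.
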(event `self.Spell`
  (`parent.Spell`)
  (`/Game/Weapons/BP_Weapon.SetCanMove` (`self.GetOwnerToMagic`) false)
  (`Character.PlayAnimMontage` (`self.GetOwnerToCharacter`) "/Game/Character/Montages/MG_Buff_Montage.MG_Buff_Montage" 1.0 "None"))

(event `self.EndSpell`
  (`parent.EndSpell`)
  (`/Game/Weapons/BP_Weapon.SetCanMove` (`self.GetOwnerToMagic`) true))

(event `self.ReceiveTick`
  (params (DeltaSeconds :type "Float (single-precision)"))
  (bind (_location _impactnormal) (`self.GetCursorLocation`)
    (:`True`
      (`SceneComponent.K2_SetWorldLocation` (`self.Decal`) _location false false)
      (`SceneComponent.K2_SetWorldRotation` (`self.Decal`) (`KismetMathLibrary.Conv_VectorToRotator` _impactnormal) false false)
      (`SceneComponent.SetVisibility` (`self.Decal`) true false))
    (:`False`
      (`SceneComponent.SetVisibility` (`self.Decal`) false false))))

(fn `UserConstructionScript`
  (`parent.UserConstructionScript`))