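; BP_Skill_Heal is a skill Blueprint that plays the casting side of a heal spell on its owning character.
; Spell runs the parent logic, disables the owner's movement through its magic interface or component, and plays a buff montage.
; EndSpell runs the parent logic and restores movement.
; No healing logic is defined here beyond what the parent class provides.
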(event `self.Spell`
  (`parent.Spell`)
  (`/Game/Weapons/BP_Weapon.SetCanMove` (`self.GetOwnerToMagic`) false)
  (`Character.PlayAnimMontage` (`self.GetOwnerToCharacter`) "/Game/Character/Montages/MG_Buff_Montage.MG_Buff_Montage" 1.0 "None"))

(event `self.EndSpell`
  (`parent.EndSpell`)
  (`/Game/Weapons/BP_Weapon.SetCanMove` (`self.GetOwnerToMagic`) true))

(fn `UserConstructionScript`
  (`parent.UserConstructionScript`))