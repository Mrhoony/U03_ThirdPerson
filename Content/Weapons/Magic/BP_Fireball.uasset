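; BP_Fireball is a magic weapon actor that deals damage to actors overlapping its collision sphere.
; On overlap it gets a single damage value from WeaponDamageComponent and passes it to SendDamage with the hit actor and a scaled-down fireball impact particle.
; SendDamage is not defined in this Blueprint, which adds no active logic beyond that overlap handler and the parent construction script call.
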(event `self.Sphere.OnComponentBeginOverlap`
  (params (OverlappedComponent :type "PrimitiveComponent Object Reference") (OtherActor :type "Actor Object Reference") (OtherComp :type "PrimitiveComponent Object Reference") (OtherBodyIndex :type Integer) (bFromSweep :type Boolean) (SweepResult :type "HitResult Structure (by ref)"))
  (bind _attack (`/Game/Components/WeaponDamageComponent.GetSingleDamage` (`self.WeaponDamageComponent`)))
  (`self.SendDamage` OtherActor _attack "/Game/Particles/P_Impact_Fireball.P_Impact_Fireball" (0.0 0.0 0.0) (0.1 0.1 0.1)))

(fn `UserConstructionScript`
  (`parent.UserConstructionScript`))