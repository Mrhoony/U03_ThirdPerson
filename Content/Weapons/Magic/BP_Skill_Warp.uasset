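; Warp skill for the magic weapon system that moves the owning character to the world point under the mouse cursor.
; While equipped, Tick places a decal and mesh marker on WorldStatic surfaces under the cursor, aligning the decal to the surface normal.
; Spell stores that point, locks movement and plays the warp montage, or ends the attack without a hit.
; A separate warp event performs a swept move above the point; EndSpell re-enables movement.
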(event `self.ReceiveBeginPlay`
  (`SceneComponent.SetVisibility` (`self.Decal`) false false)
  (`SceneComponent.SetVisibility` (`self.StaticMesh`) false false))

(event `self.OnEquipped`
  (`parent.OnEquipped`)
  (set `self.Equipped` true))

(event `self.OnUnequipped`
  (`parent.OnUnequipped`)
  (set `self.Equipped` false))

(event `self.Spell`
  (`parent.Spell`)
  (bind _location (`self.GetCursorLocation`)
    (:`True`
      (set `self.WarpLocation` _location)
      (set `self.CanWarp` true)
      (`/Game/Weapons/BP_Weapon.SetCanMove` (`self.GetOwnerToMagic`) false)
      (`Character.PlayAnimMontage` (`self.GetOwnerToCharacter`) "/Game/Character/Montages/MG_Warp_Montage.MG_Warp_Montage" 2.0 "None"))
    (:`False`
      (`/Game/Weapons/BP_Weapon.EndAttack` (`self.GetOwnerToMagic`))
      (set `self.CanWarp` false))))

(event `self.EndSpell`
  (`parent.EndSpell`)
  (`/Game/Weapons/BP_Weapon.SetCanMove` (`self.GetOwnerToMagic`) true))

(event `self.ReceiveTick`
  (params (DeltaSeconds :type "Float (single-precision)"))
  (if (`self.Equipped`)
    (bind (_location _impactnormal) (`self.GetCursorLocation`)
      (:`True`
        (`SceneComponent.K2_SetWorldLocation` (`self.Decal`) _location false false)
        (`SceneComponent.K2_SetWorldLocation` (`self.StaticMesh`) _location false false)
        (`SceneComponent.K2_SetWorldRotation` (`self.Decal`) (`KismetMathLibrary.Conv_VectorToRotator` _impactnormal) false false)
        (`SceneComponent.SetVisibility` (`self.Decal`) true false)
        (`SceneComponent.SetVisibility` (`self.StaticMesh`) true false))
      (:`False`
        (`SceneComponent.SetVisibility` (`self.Decal`) false false :!label _label)
        (`SceneComponent.SetVisibility` (`self.StaticMesh`) false false)))
    (else
      (goto _label))))

(event `warp`
  (if (`self.CanWarp`)
    (set `self.CanWarp` false)
    (bind (_sweephitresult _returnvalue) (`self.K2_SetActorLocation` (`self.GetOwnerToCharacter`) (`KismetMathLibrary.MakeVector` (.x (`self.WarpLocation`)) (.y (`self.WarpLocation`)) (+ (.z (`self.WarpLocation`)) 200.0)) true false))
    (if _returnvalue
      (`KismetSystemLibrary.PrintString` (`KismetSystemLibrary.GetDisplayName` (`.HitComponent` (`GameplayStatics.BreakHitResult` _sweephitresult)))))))

(fn `UserConstructionScript`
  (`parent.UserConstructionScript`))