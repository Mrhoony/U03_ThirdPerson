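; BP_ThrowItem is a thrown magic projectile actor that lives for a few seconds and uses a fireball impact effect.
; When its Sphere overlaps an actor, SendDamage spawns the impact particle, oriented from the caster toward that actor, then destroys the item.
; Damage is forwarded to BP_Magic, found through the owner chain: item to BP_Skill_Throw to BP_Magic, whose owner serves as caster.
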(event `self.ReceiveBeginPlay`
  (`self.SetLifeSpan` 3.0))

(event `self.Sphere.OnComponentBeginOverlap`
  (params (OverlappedComponent :type "PrimitiveComponent Object Reference") (OtherActor :type "Actor Object Reference") (OtherComp :type "PrimitiveComponent Object Reference") (OtherBodyIndex :type Integer) (bFromSweep :type Boolean) (SweepResult :type "HitResult Structure (by ref)"))
  (`self.SendDamage` OtherActor 20.0 "/Game/Particles/P_Impact_Fireball.P_Impact_Fireball"))

(fn `GetOwnerToMagic`
  (returns (`AsBP Magic` :type "/Game/Weapons/Magic/BP_Magic Object Reference"))
  (bind _asbp_magic (cast `/Game/Weapons/Magic/BP_Magic` (`self.GetOwner` (`self.GetOwnerToThrow`))))
  (return _asbp_magic))

(fn `GetOwnerToThrow`
  (returns (`AsBP Skill Throw` :type "/Game/Weapons/Magic/BP_Skill_Throw Object Reference"))
  (bind _asbp_skill_throw (cast `/Game/Weapons/Magic/BP_Skill_Throw` (`self.GetOwner`)))
  (return _asbp_skill_throw))

(fn `SendDamage`
  (params (OtherActor :type "Actor Object Reference") (Damage :type "Float (double-precision)" :default 20.0) (ImpactParticle :type "ParticleSystem Object Reference") (ImpactParticleOffset :type "Vector Structure") (ImpactParticleScale :type "Vector Structure" :default (1.0 1.0 1.0)))
  (`GameplayStatics.SpawnEmitterAtLocation` (`local.ImpactParticle`) (+ (`self.K2_GetActorLocation`) (`local.ImpactParticleOffset`)) (`KismetMathLibrary.FindLookAtRotation` (`self.K2_GetActorLocation` (`self.GetOwner` (`self.GetOwnerToMagic`))) (`self.K2_GetActorLocation` (`local.OtherActor`))) (`local.ImpactParticleScale`))
  (`/Game/Weapons/BP_Weapon.SendDamage` (`self.GetOwnerToMagic`) (`local.OtherActor`) (`local.Damage`))
  (`self.K2_DestroyActor`))

(fn `UserConstructionScript`)