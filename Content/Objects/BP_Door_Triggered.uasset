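; Triggered double sliding door with a rotating lock, opened by an external OpenDoor event and shut when the player enters its box.
; Events check an Opened flag, then chained timelines spin the lock and slide both panels apart, or close the panels before turning the lock.
; The box disables its collision after the first player overlap, so that automatic close happens only once.
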(event `OpenDoor`
  (if (not (`self.Opened`))
    (set `self.Opened` true)
    (bind (_direction _speed) (`Timeline|LockOpen` :!via `PlayFromStart`)
      (:`Update`
        (`SceneComponent.K2_SetRelativeRotation` (`self.Lock`) (`KismetMathLibrary.MakeRotator` (* _speed 720.0)) false false))
      (:`Finished`
        (bind (_direction_2 _speed_2) (`Timeline|DoorOpen` :!via `PlayFromStart`)
          (:`Update`
            (bind _returnvalue (`KismetMathLibrary.MakeVector` 0.0 (* _speed_2 260.0)))
            (`SceneComponent.K2_SetRelativeLocation` (`self.RightDoor`) _returnvalue false false)
            (`SceneComponent.K2_SetRelativeLocation` (`self.LeftDoor`) (* _returnvalue -1.0) false false)))))))

(event `self.ReceiveTick`
  (params (DeltaSeconds :type "Float (single-precision)")))

(event `CloseDoor`
  (if (`self.Opened`)
    (set `self.Opened` false)
    (bind (_direction _speed) (`Timeline|DoorClose` :!via `PlayFromStart`)
      (:`Update`
        (bind _returnvalue (`KismetMathLibrary.MakeVector` 0.0 (* _speed 260.0)))
        (`SceneComponent.K2_SetRelativeLocation` (`self.RightDoor`) _returnvalue false false)
        (`SceneComponent.K2_SetRelativeLocation` (`self.LeftDoor`) (* _returnvalue -1.0) false false))
      (:`Finished`
        (bind (_direction_2 _speed_2) (`Timeline|LockClose` :!via `PlayFromStart`)
          (:`Update`
            (`SceneComponent.K2_SetRelativeRotation` (`self.Lock`) (`KismetMathLibrary.MakeRotator` (* _speed_2 720.0)) false false)))))))

(event `self.Box.OnComponentBeginOverlap`
  (params (OverlappedComponent :type "PrimitiveComponent Object Reference") (OtherActor :type "Actor Object Reference") (OtherComp :type "PrimitiveComponent Object Reference") (OtherBodyIndex :type Integer) (bFromSweep :type Boolean) (SweepResult :type "HitResult Structure (by ref)"))
  (cast `/Game/Player/BP_Player` OtherActor)
  (`self.CloseDoor`)
  (`PrimitiveComponent.SetCollisionEnabled` (`self.Box`) "NoCollision"))

(fn `UserConstructionScript`)