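; BP_Sister is a player-controlled character with camera-relative movement, jumping, walk-speed switching and a sword that draws and holsters.
; Equip and unequip lock movement and swap rotation mode, while separate events move the sword between hand and holster sockets and finish each transition.
; A drawn sword allows a montage attack, gated until EndAttack.
; X triggers an upward-pushed ragdoll that quits the game after a delay; sword spawning and camera switching are unwired.
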(fn `UserConstructionScript`)