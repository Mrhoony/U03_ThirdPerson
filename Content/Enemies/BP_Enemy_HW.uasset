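; Enemy actor that patrols or jumps in place until a sword knocks it into a ragdoll.
; On BeginPlay it holsters a spawned BP_GreatSword, then AIState selects a delayed loop between its start and GoalPoint, or repeated jumping.
; Capsule overlap with BP_Sword disables capsule collision, enables mesh physics and pushes it along the wielder's forward vector.
; The hit also sets IsRagDoll to end the loop and calls Clear on ClearEvent.
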(event `self.ReceiveBeginPlay`
  (bind _delay (`self.Delay`))
  ;[1 1 1] 코멘트
  (bind _returnvalue (`|SpawnActorFromClass` "/Game/Weapons/Melee/BP_GreatSword.BP_GreatSword_C" (`KismetMathLibrary.MakeTransform` (0.0 0.0 0.0)) "Undefined" "OverrideRootScale" self null))
  (bind _output_get (set `self.GreatSword` _returnvalue))
  (`self.K2_AttachToComponent` _output_get (`self.Mesh`) "Holster_GreatSword" "KeepRelative" "KeepRelative" "KeepRelative" true)
  (switch `/Game/Enums/EAIStateType` (`self.AIState`)
    (:`NewEnumerator0`
      (set `self.ReturnPoint` (`self.K2_GetActorLocation`))
      (`AIBlueprintHelperLibrary.SimpleMoveToLocation` (`self.GetController` self) (`self.K2_GetActorLocation` (`self.GoalPoint`)) :!label _label)
      (`KismetSystemLibrary.Delay` _delay)
      (`AIBlueprintHelperLibrary.SimpleMoveToLocation` (`self.GetController` self) (`self.ReturnPoint`))
      (`KismetSystemLibrary.Delay` _delay)
      (if (not (`self.IsRagDoll`))
        (goto _label)))
    (:`NewEnumerator1`
      (`self.Jump` self :!label _label_2)
      (`KismetSystemLibrary.Delay` (`self.Delay`))
      (if (not (`self.IsRagDoll`))
        (goto _label_2)))))

(event `self.CapsuleComponent.OnComponentBeginOverlap`
  (params (OverlappedComponent :type "PrimitiveComponent Object Reference") (OtherActor :type "Actor Object Reference") (OtherComp :type "PrimitiveComponent Object Reference") (OtherBodyIndex :type Integer) (bFromSweep :type Boolean) (SweepResult :type "HitResult Structure (by ref)"))
  (bind _mesh (`self.Mesh`))
  ;[1 1 1] 코멘트
  (bind _asbp_sword (cast `/Game/Weapons/Melee/BP_Sword` OtherActor))
  (`PrimitiveComponent.SetCollisionEnabled` (`self.CapsuleComponent`) "NoCollision")
  (set `SkeletalMeshComponent.GlobalAnimRateScale` 0.0 _mesh)
  (`PrimitiveComponent.SetSimulatePhysics` _mesh true)
  (`PrimitiveComponent.SetCollisionEnabled` _mesh "QueryAndPhysics")
  (`PrimitiveComponent.AddForce` _mesh (* (`self.GetActorForwardVector` (`self.GetAttachParentActor` _asbp_sword)) 5000000.0) "None" false)
  (set `self.IsRagDoll` true)
  (`/Game/Demo/BP_Stage3_Clear.Clear` (`self.ClearEvent`)))

(fn `UserConstructionScript`)